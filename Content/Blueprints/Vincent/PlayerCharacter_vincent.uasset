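; Player character Blueprint for a sword-wielding fighter with simple and special attacks, potion, regeneration and strength aura.
; Character events set attack flags, start cooldowns on actors found by class, and spawn hit, regen and aura effects.
; BeginPlay attaches a gladius and blade collider to the weapon socket; Tick resizes the lifebar, moves effects and pulses special-charge flags.
; It also updates the overhead name, toggles HUD sections and binds debug keys for speed, gamma and resolution.
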(event `self.CharacterAttackedSimple`
  ;[1 1 1] Attack Simple
  (set `self.IsSimpleAttacking` true)
  (`|ExecutionSequence`
    (:`then_0`
      (set `self.ISAttackPressed_Player` true)
      (`KismetSystemLibrary.Delay` 0.2)
      (set `self.ISAttackPressed_Player` false))
    (:`then_1`
      (bind _outactors (`GameplayStatics.GetAllActorsOfClass` "/Game/UI/HUD/Cooldowns/Cooldown_SimpleAttack.Cooldown_SimpleAttack_C"))
      (for _array_element _outactors
        (bind _ascooldown_simpleattack_c (cast `/Game/UI/HUD/Cooldowns/Cooldown_SimpleAttack` _array_element))
        (`/Game/UI/HUD/Cooldowns/Cooldown_SimpleAttack.StartCooldown_SimpleAttack` _ascooldown_simpleattack_c (`self.SimpleAttackCoolDown`))))))

(event `CallSetIsSimpleAttackingTo`
  (params (Value :type Boolean))
  ;[1 1 1] Attack Simple
  (`self.SetIsSimpleAttackingTo` Value))

(event `self.CharacterAppliedSimpleForce`
  ;[1 1 1] Attack Simple
)

(event `self.CharacterAttackedSpecial`
  ;[1 1 1] Attack Special
  (`|ExecutionSequence`
    (:`then_0`
      (bind _outactors (`GameplayStatics.GetAllActorsOfClass` "/Game/UI/HUD/Cooldowns/Cooldown_SpecialAttack.Cooldown_SpecialAttack_C"))
      (for _array_element _outactors
        (bind _ascooldown_specialattack_c (cast `/Game/UI/HUD/Cooldowns/Cooldown_SpecialAttack` _array_element))
        (`/Game/UI/HUD/Cooldowns/Cooldown_SpecialAttack.StartCooldown_SpecialAttack` _ascooldown_specialattack_c (`self.SpecialAttackCoolDown`))))))

(event `CallSetIsSpecialAttackingTo`
  (params (Value :type Boolean))
  ;[1 1 1] Attack Special
  (`self.SetIsSpecialAttackingTo` Value))

(event `self.CharacterAppliedSpecialForce`
  ;[1 1 1] Attack Special
)

(event `self.CharacterUsedPotion`
  ;[1 1 1] Potion
)

(event `InputAction|UsePotion`
  ;[1 1 1] Potion
  (:`Pressed`
    (bind _outactors (`GameplayStatics.GetAllActorsOfClass` "/Game/UI/HUD/Cooldowns/Cooldown_Potion.Cooldown_Potion_C"))
    (for _array_element _outactors
      (bind _ascooldown_potion_c (cast `/Game/UI/HUD/Cooldowns/Cooldown_Potion` _array_element))
      (`/Game/UI/HUD/Cooldowns/Cooldown_Potion.StartCooldown_Potion` _ascooldown_potion_c (`self.PotionCoolDown`)))))

(event `self.CharacterFinishedRegeneration`
  ;[1 1 1] Regen
  (`ActorComponent.K2_DestroyComponent` (`self.SpawnedRegen`)))

(event `self.CharacterStartedRegeneration`
  ;[1 1 1] Regen
  (`/Engine/EditorBlueprintResources/StandardMacros.IsValid` "/Game/VFX/Particles/P_Regen.P_Regen"
    (:`Is Valid`
      (bind _returnvalue (`GameplayStatics.SpawnEmitterAtLocation` "/Game/VFX/Particles/P_Regen.P_Regen" (+ (`self.K2_GetActorLocation`) (0.0 0.0 30.0))))
      (set `self.SpawnedRegen` _returnvalue))))

(event `DisableAllScreenMessages`
  ;[1 0.886 0.3546] TOOLS
  ;;[1 1 1] Disable Screen Messages
  (`KismetSystemLibrary.ExecuteConsoleCommand` "disableallscreenmessages"))

(event `Key|PageUp`
  ;[1 0.886 0.3546] TOOLS
  ;;[1 1 1] Restoggle
  (:`Pressed`
    (set `self.Increase?` true)
    (`self.Setresxy` (`self.Increase?`) :!label _label)))

(event `self.ReceiveTick`
  (params (DeltaSeconds :type "Float (single-precision)"))
  (bind _lifebar (`self.Lifebar`))
  ;[1 0.4045 0.8106] TICK
  (`|ExecutionSequence`
    (:`then_0`
      ;[1 1 1] Set current lifebar size
      (bind _asgacharacter (cast `GACharacter` (`GameplayStatics.GetPlayerCharacter` 0)))
      (`KismetArrayLibrary.Array_Set` (`MaterialBillboardComponent.Elements` (`self.Lifebar`)) 0 (make `MaterialBillboardComponent.MaterialSpriteElement` "/Game/VFX/_VFX_Shader/healthbar.healthbar" null false 8.0 (* (/ (`GACharacter.HealthPoints` _asgacharacter) (`GACharacter.MaxHealth` _asgacharacter)) 32.0)) true)
      (`SceneComponent.ToggleVisibility` _lifebar true)
      (`SceneComponent.ToggleVisibility` _lifebar false))
    (:`then_1`
      ;[1 1 1] Regen
      (`/Engine/EditorBlueprintResources/StandardMacros.IsValid` "/Game/VFX/Particles/P_Regen.P_Regen"
        (:`Is Valid`
          (`SceneComponent.SetWorldLocation` (`self.SpawnedRegen`) (0.0 0.0 0.0) false))))
    (:`then_2`
      ;[1 1 1] Aura
      (`/Engine/EditorBlueprintResources/StandardMacros.IsValid` (stale `self.CharacterActivatedAura` _returnvalue)
        (:`Is Valid`
          (`self.K2_SetActorLocation` (stale `self.CharacterActivatedAura` _returnvalue) (- (`self.K2_GetActorLocation`) (0.0 0.0 50.0)) false))))
    (:`then_3`
      ;[1 1 1] Attack Special
      (`|ExecutionSequence`
        (:`then_0`
          (if (not (`self.IsSpecialCooldown_Player`))
            (bind _returnvalue (`self.IsCharging`))
            (set `self.IsSpecialCharging_Player` _returnvalue)))
        (:`then_1`
          (if (`self.IsSpecialCooldown_Player`)
            _
            (elif (`self.IsSpecialCharging_Player`)
              (set `self.IsSpecialAttackPressed_Player` true)
              (`KismetSystemLibrary.Delay` 0.1)
              (set `self.IsSpecialAttackPressed_Player` false))))))))

(event `CharacterTookDamage`
  ;[1 1 1] Take_Damage
  (`GameplayStatics.SpawnEmitterAtLocation` "/Game/VFX/Particles/Particle_Hit.Particle_Hit" (`self.GetPlayerForwardVector` -5.0 (0.0 0.0 10.0))))

(event `Key|PageDown`
  ;[1 0.886 0.3546] TOOLS
  ;;[1 1 1] Restoggle
  (:`Pressed`
    (set `self.Increase?` false)
    (goto _label)))

(event `Key|MouseScrollDown`
  (bind _charactermovement (`self.CharacterMovement`))
  ;[1 0.886 0.3546] TOOLS
  ;;[1 1 1] MovespeedMod
  (:`Pressed`
    (set `CharacterMovementComponent.MaxWalkSpeed` (`KismetMathLibrary.FClamp` (+ (`CharacterMovementComponent.MaxWalkSpeed` _charactermovement) -500.0) 100.0 5000.0) _charactermovement)))

(event `Key|Add`
  ;[1 0.886 0.3546] TOOLS
  ;;[1 1 1] Brightnesscontrol
  (:`Pressed`
    (`self.Gamma+` (`self.Increment`))))

(event `self.ReceiveBeginPlay`
  ;[1 0.4045 0.8106] BeginPlay
  (`|ExecutionSequence`
    (:`then_0`
      ;[1 1 1] Equip Sword
      (bind _returnvalue (`|SpawnActorFromClass` "/Game/Blueprints/Peddy/Items/bp_weapon_gladius.bp_weapon_gladius_C" (`KismetMathLibrary.MakeTransform` (0.0 0.0 0.0) (struct) (2.54 2.54 2.54)) true))
      (bind _asgacharacter (cast `GACharacter` (`self.GetInstigator`)))
      (`GAWeapon.SetNewOwner` _returnvalue _asgacharacter)
      (`self.AttachRootComponentTo` _returnvalue (`self.Mesh`) "Weapon" "KeepRelativeOffset"))
    (:`then_1`
      ;[0.3615 0.1646 0.37] Remote Events
      (`self.MC_DisableAllScreenMessages`))
    (:`then_2`
      (`SceneComponent.AttachTo` (`self.Collider_Weapon_Blade`) (`self.Mesh`) "Weapon" "KeepRelativeOffset"))))

(event `Key|MouseScrollUp`
  (bind _charactermovement (`self.CharacterMovement`))
  ;[1 0.886 0.3546] TOOLS
  ;;[1 1 1] MovespeedMod
  (:`Pressed`
    (set `CharacterMovementComponent.MaxWalkSpeed` (`KismetMathLibrary.FClamp` (+ (`CharacterMovementComponent.MaxWalkSpeed` _charactermovement) 500.0) 100.0 5100.0) _charactermovement)))

(event `Key|Subtract`
  ;[1 0.886 0.3546] TOOLS
  ;;[1 1 1] Brightnesscontrol
  (:`Pressed`
    (`self.Gamma-` (`self.Increment`))))

(event `Key|MiddleMouseButton`
  ;[1 0.886 0.3546] TOOLS
  ;;[1 1 1] MovespeedMod
  (:`Pressed`
    (set `CharacterMovementComponent.MaxWalkSpeed` 600.0 (`self.CharacterMovement`))))

(event `self.CharacterActivatedAura`
  ;[1 1 1] Aura
  (bind _returnvalue (`|SpawnActorFromClass` "/Game/VFX/BP_Aura_Strength.BP_Aura_Strength_C" (`KismetMathLibrary.MakeTransform` (- (`self.K2_GetActorLocation`) (0.0 0.0 50.0))) true)))

(event `self.CharacterDeactivatedAura`
  ;[1 1 1] Aura
  (`/Engine/EditorBlueprintResources/StandardMacros.IsValid` (stale `self.CharacterActivatedAura` _returnvalue)
    (:`Is Valid`
      (`self.K2_DestroyActor` (stale `self.CharacterActivatedAura` _returnvalue)))))

(event `Key|Z`
  ;[1 1 1] Destroy_Heart
  (:`Pressed`
    (`/Engine/EditorBlueprintResources/StandardMacros.IsValid` "/Game/VFX/Shard/BP_Mockup_Shard_DM.BP_Mockup_Shard_DM"
      (:`Is Valid`
        (bind _outactors (`GameplayStatics.GetAllActorsOfClass` "/Game/VFX/Shard/BP_Mockup_Shard_DM.BP_Mockup_Shard_DM_C"))
        (for _array_element _outactors
          (bind _asbp_mockup_shard_dm_c (cast `/Game/VFX/Shard/BP_Mockup_Shard_DM` _array_element))
          (`/Game/VFX/Shard/BP_Mockup_Shard_DM.Destroy_Heart` _asbp_mockup_shard_dm_c))))))

(event `self.CharacterChangedName`
  ;[1 1 1] Update Namechange
  (`self.UpdateTextRenderer`))

(event `Key|I`
  ;[1 1 1] Toggle inventory
  (:`Pressed`
    (bind _asga_hud_bp_c (cast `/Game/UI/Classes/GA_HUD_BP` (`PlayerController.GetHUD` (`GameplayStatics.GetPlayerController` 0))))
    (bind _returnvalue (`GA_HUD.getSection` _asga_hud_bp_c "inventory"))
    (switch `int` _returnvalue
      (:`0`
        (set `self.showInventory` true))
      (:`1`
        (set `self.showInventory` false)))
    (`GA_HUD.toggleSection` _asga_hud_bp_c "inventory" (`self.showInventory`))))

(event `Key|Z`
  ;[1 1 1] Toggle escapemenu
  (:`Pressed`
    (bind _asga_hud_bp_c (cast `/Game/UI/Classes/GA_HUD_BP` (`PlayerController.GetHUD` (`GameplayStatics.GetPlayerController` 0))))
    (bind _returnvalue (`GA_HUD.getSection` _asga_hud_bp_c "escapemenu"))
    (switch `int` _returnvalue
      (:`0`
        (set `self.showEscapemenu` true))
      (:`1`
        (set `self.showEscapemenu` false)))
    (`GA_HUD.toggleSection` _asga_hud_bp_c "escapemenu" (`self.showEscapemenu`))))

(event `Key|P`
  ;[1 1 1] Toggle stats
  (:`Pressed`
    (set `self.showStats` true)
    (bind _asga_hud_bp_c (cast `/Game/UI/Classes/GA_HUD_BP` (`PlayerController.GetHUD` (`GameplayStatics.GetPlayerController` 0)) :!label _label_2))
    (`GA_HUD.toggleSection` _asga_hud_bp_c "sessioninfo" (`self.showStats`)))
  (:`Released`
    (set `self.showStats` false)
    (goto _label_2)))

(fn `Gamma+`
  (params (Increment :type "Float (double-precision)"))
  (set `self.Gamma` (`KismetMathLibrary.FClamp` (+ (`self.Gamma`) (`self.Increment`)) 0.2 4.2))
  (`KismetSystemLibrary.ExecuteConsoleCommand` (`KismetStringLibrary.Concat_StrStr` "gamma " (`KismetStringLibrary.Conv_DoubleToString` (`self.Gamma`)))))

(fn `Gamma-`
  (params (Increment :type "Float (double-precision)"))
  (set `self.Gamma` (`KismetMathLibrary.FClamp` (- (`self.Gamma`) (`self.Increment`)) 0.2 4.2))
  (`KismetSystemLibrary.ExecuteConsoleCommand` (`KismetStringLibrary.Concat_StrStr` "gamma " (`KismetStringLibrary.Conv_DoubleToString` (`self.Gamma`)))))

(fn `OnRep_Special_IsCharging`)

(fn `Setresxy`
  (params (`Increase/Decrease` :type Boolean))
  (bind _returnvalue (`KismetStringLibrary.Concat_StrStr` "setres " (`self.1920x1200`)))
  (bind _returnvalue_2 (`KismetStringLibrary.Concat_StrStr` "setres " (`self.1920x1080`)))
  (if true
    (`KismetSystemLibrary.ExecuteConsoleCommand` _returnvalue (`GameplayStatics.GetPlayerController` 0))
    (set `self.Resolution` _returnvalue)
    (else
      (`KismetSystemLibrary.ExecuteConsoleCommand` _returnvalue_2 (`GameplayStatics.GetPlayerController` 0))
      (set `self.Resolution` _returnvalue_2))))

(fn `UpdateTextRenderer`
  ;[1 1 1] Update textrenderer above player mesh
  (`TextRenderComponent.SetText` (`self.UsernameRenderer`) (`self.UserName`))
  (return))

(fn `UserConstructionScript`
  (`self.UpdateTextRenderer`))