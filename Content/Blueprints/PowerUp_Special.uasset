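; PowerUp_Special is a child power-up pickup whose look follows PowerUpType, with invulnerability and one-hit variants besides the default type.
; The construction script runs the parent's logic, enlarges the mesh, and sets mesh and particle material for the two non-default types.
; When cooldown finishes, the event reapplies those visuals, including the one-hit mesh material that construction omits, and tints the light per type.
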(event `self.PowerUpFinishedCoolDown`
  (bind _poweruptype (`self.PowerUpType`))
  (bind _powerup_mesh (`self.PowerUp_Mesh`))
  (bind _poweruptype_2 (`self.PowerUpType`))
  (bind _light (`self.Light`))
  (`|ExecutionSequence`
    (:`then_0`
      (if (== _poweruptype 1)
        (`StaticMeshComponent.SetStaticMesh` _powerup_mesh "/Game/Meshes/Items/item_armor_helmet.item_armor_helmet")
        (`PrimitiveComponent.SetMaterial` _powerup_mesh 0 "/Game/VFX/_VFX_Shader/_VFX_Instances/invul.invul")
        (`PrimitiveComponent.SetMaterial` (`self.AmbientParticle`) 0 "/Game/VFX/_VFX_Shader/_VFX_Instances/Particle_Pod_ambient2.Particle_Pod_ambient2")
        (elif (== _poweruptype 2)
          (`StaticMeshComponent.SetStaticMesh` _powerup_mesh "/Game/Meshes/SG_powerup_onehit.SG_powerup_onehit")
          (`PrimitiveComponent.SetMaterial` _powerup_mesh 0 "/Game/VFX/_VFX_Shader/_VFX_Instances/onehit.onehit")
          (`PrimitiveComponent.SetMaterial` (`self.AmbientParticle`) 0 "/Game/VFX/_VFX_Shader/_VFX_Instances/Particle_Pod_ambient.Particle_Pod_ambient"))))
    (:`then_1`
      (if (== _poweruptype_2 0)
        (`LightComponent.SetLightColor` _light (struct :`R` 0.299925 :`G` 0.995 :`B` 0.192991 :`A` 1.0))
        (elif (== _poweruptype_2 1)
          (`LightComponent.SetLightColor` _light (struct :`R` 0.995 :`G` 0.814951 :`B` 0.213925 :`A` 1.0))
          (elif (== _poweruptype_2 2)
            (`LightComponent.SetLightColor` _light (struct :`R` 0.192991 :`G` 0.292421 :`B` 0.995 :`A` 1.0))))))))

(fn `UserConstructionScript`
  (bind _poweruptype (`self.PowerUpType`))
  (bind _powerup_mesh (`self.PowerUp_Mesh`))
  (`parent.UserConstructionScript`)
  (`SceneComponent.SetWorldScale3D` _powerup_mesh (2.0 2.0 2.0))
  (if (== _poweruptype 1)
    (`StaticMeshComponent.SetStaticMesh` _powerup_mesh "/Game/Meshes/Items/item_armor_helmet.item_armor_helmet")
    (`PrimitiveComponent.SetMaterial` _powerup_mesh 0 "/Game/VFX/_VFX_Shader/_VFX_Instances/invul.invul")
    (`PrimitiveComponent.SetMaterial` (`self.AmbientParticle`) 0 "/Game/VFX/_VFX_Shader/_VFX_Instances/Particle_Pod_ambient2.Particle_Pod_ambient2")
    (elif (== _poweruptype 2)
      (`StaticMeshComponent.SetStaticMesh` _powerup_mesh "/Game/Meshes/SG_powerup_onehit.SG_powerup_onehit")
      (`PrimitiveComponent.SetMaterial` (`self.AmbientParticle`) 0 "/Game/VFX/_VFX_Shader/_VFX_Instances/Particle_Pod_ambient.Particle_Pod_ambient"))))