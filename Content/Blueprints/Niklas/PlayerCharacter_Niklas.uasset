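; Player character Blueprint that adds particle feedback for combat events, plus test-style input for movement speed and shard hearts.
; Attack, damage and regeneration events spawn emitters offset from player 0, with attacks oriented by mesh yaw.
; Tick keeps the regeneration emitter on the player and calls AA on every Sword found in the world.
; Mouse wheel and middle button adjust or reset walk speed, while Z calls DestroyHeart on all mockup shards.
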(event `Key|MouseScrollDown`
  (bind _charactermovement (`self.CharacterMovement`))
  (:`Pressed`
    (set `CharacterMovementComponent.MaxWalkSpeed` (`KismetMathLibrary.FClamp` (+ (`CharacterMovementComponent.MaxWalkSpeed` _charactermovement) -500.0) 100.0 5000.0) _charactermovement)))

(event `Key|MouseScrollUp`
  (bind _charactermovement (`self.CharacterMovement`))
  (:`Pressed`
    (set `CharacterMovementComponent.MaxWalkSpeed` (`KismetMathLibrary.FClamp` (+ (`CharacterMovementComponent.MaxWalkSpeed` _charactermovement) 500.0) 100.0 5100.0) _charactermovement)))

(event `Key|MiddleMouseButton`
  (:`Pressed`
    (set `CharacterMovementComponent.MaxWalkSpeed` 600.0 (`self.CharacterMovement`))))

(event `self.CharacterAttackedSimple`
  ;[1 0 0] EVENTS
  ;;[1 1 1] Attack_Standard
  (`/Engine/EditorBlueprintResources/StandardMacros.IsValid` "PlayerCharacter_Niklas"
    (:`Is Valid`
      (bind _returnvalue (`GameplayStatics.SpawnEmitterAtLocation` "/Game/VFX/Particles/Particle_Attack_Basic.Particle_Attack_Basic" (+ (* (`KismetMathLibrary.GetForwardVector` (`KismetMathLibrary.MakeRot` 0.0 (- (.yaw (`SceneComponent.K2_GetComponentRotation` (`self.Mesh`))) -90.0) (- (.roll (`SceneComponent.K2_GetComponentRotation` (`self.Mesh`))) -90.0))) 30.0) (+ (`self.K2_GetActorLocation` (`GameplayStatics.GetPlayerCharacter` 0)) (0.0 0.0 20.0))) (`KismetMathLibrary.MakeRot` 0.0 (- (.yaw (`SceneComponent.K2_GetComponentRotation` (`self.Mesh`))) -90.0) (- (.roll (`SceneComponent.K2_GetComponentRotation` (`self.Mesh`))) -90.0))))
      (set `self.Spawnedparticle` _returnvalue))))

(event `self.ReceiveTick`
  (params (DeltaSeconds :type "Float (single-precision)"))
  (`|ExecutionSequence`
    (:`then_0`
      (`/Engine/EditorBlueprintResources/StandardMacros.IsValid` "/Game/VFX/Particles/P_Regen.P_Regen"
        (:`Is Valid`
          (`SceneComponent.SetWorldLocation` (`self.SpawnedRegen`) (+ (+ (+ (`self.K2_GetActorLocation` (`GameplayStatics.GetPlayerCharacter` 0)) (0.0 0.0 20.0)) (* (`KismetMathLibrary.GetForwardVector` (`KismetMathLibrary.MakeRot` 0.0 (- (.yaw (`SceneComponent.K2_GetComponentRotation` (`self.Mesh`))) -90.0) (- (.roll (`SceneComponent.K2_GetComponentRotation` (`self.Mesh`))) -90.0))) -5.0)) (0.0 0.0 10.0)) false))))
    (:`then_1`
      (bind _outactors (`GameplayStatics.GetAllActorsOfClass` "/Game/Blueprints/Items/Sword.Sword_C"))
      (for _array_element _outactors
        (bind _assword_c (cast `/Game/Blueprints/Items/Sword` _array_element))
        (`/Game/Blueprints/Items/Sword.AA` _assword_c)))))

(event `self.CharacterAttackedSpecial`
  ;[1 0 0] EVENTS
  ;;[1 1 1] Attack_Charged
  (`/Engine/EditorBlueprintResources/StandardMacros.IsValid` "PlayerCharacter_Niklas"
    (:`Is Valid`
      (bind _returnvalue (`GameplayStatics.SpawnEmitterAtLocation` "/Game/VFX/Particles/Particle_Attack_Charged.Particle_Attack_Charged" (+ (`self.K2_GetActorLocation` (`GameplayStatics.GetPlayerCharacter` 0)) (0.0 0.0 20.0)) (`KismetMathLibrary.MakeRot` 0.0 (- (.yaw (`SceneComponent.K2_GetComponentRotation` (`self.Mesh`))) -90.0) (- (.roll (`SceneComponent.K2_GetComponentRotation` (`self.Mesh`))) -90.0))))
      (set `self.Spawnedparticle` _returnvalue))))

(event `self.CharacterFinishedRegeneration`
  (`ActorComponent.K2_DestroyComponent` (`self.SpawnedRegen`)))

(event `self.CharacterStartedRegeneration`
  ;[1 0 0] EVENTS
  ;;[1 1 1] Regen
  (`/Engine/EditorBlueprintResources/StandardMacros.IsValid` "/Game/VFX/Particles/P_Regen.P_Regen"
    (:`Is Valid`
      (bind _returnvalue (`GameplayStatics.SpawnEmitterAtLocation` "/Game/VFX/Particles/P_Regen.P_Regen" (+ (`self.K2_GetActorLocation` (`GameplayStatics.GetPlayerCharacter` 0)) (0.0 0.0 30.0))))
      (set `self.SpawnedRegen` _returnvalue))))

(event `self.CharacterTookDamage`
  ;[1 0 0] EVENTS
  ;;[1 1 1] Take_Damage
  (`/Engine/EditorBlueprintResources/StandardMacros.IsValid` "/Game/VFX/Particles/P_Regen.P_Regen"
    (:`Is Valid`
      (`GameplayStatics.SpawnEmitterAtLocation` "/Game/VFX/Particles/Particle_Hit.Particle_Hit" (+ (+ (+ (`self.K2_GetActorLocation` (`GameplayStatics.GetPlayerCharacter` 0)) (0.0 0.0 20.0)) (* (`KismetMathLibrary.GetForwardVector` (`KismetMathLibrary.MakeRot` 0.0 (- (.yaw (`SceneComponent.K2_GetComponentRotation` (`self.Mesh`))) -90.0) (- (.roll (`SceneComponent.K2_GetComponentRotation` (`self.Mesh`))) -90.0))) -5.0)) (0.0 0.0 10.0))))))

(event `Key|Z`
  ;[1 0 0] EVENTS
  ;;[1 1 1] Destroy_Heart
  (:`Pressed`
    (`/Engine/EditorBlueprintResources/StandardMacros.IsValid` "/Game/VFX/BP_Mockup_Shard_DM.BP_Mockup_Shard_DM"
      (:`Is Valid`
        (bind _outactors (`GameplayStatics.GetAllActorsOfClass` "/Game/VFX/BP_Mockup_Shard_DM.BP_Mockup_Shard_DM_C"))
        (for _array_element _outactors
          (bind _asbp_mockup_shard_dm_c (cast `/Game/VFX/BP_Mockup_Shard_DM` _array_element))
          (`/Game/VFX/BP_Mockup_Shard_DM.Destroy_Heart` _asbp_mockup_shard_dm_c))))))

(fn `UserConstructionScript`)