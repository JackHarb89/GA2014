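; Small enemy Blueprint with example handlers for damage and death, plus a hit effect.
; The damage event prints the amount and passes it to ApplyDamage, while the death event prints a message and calls DoDeath.
; A separate CharacterTookDamage event spawns an enlarged hit particle slightly above the mesh's location.
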(event `self.CharacterHasTakenDamage`
  (params (Damage :type "Float (single-precision)"))
  ;[0 0.5356 1] Example damagehandler
  (`KismetSystemLibrary.PrintString` (`KismetStringLibrary.Concat_StrStr` "Bam! Enemy took damage: " (`KismetStringLibrary.Conv_DoubleToString` Damage)))
  (`self.ApplyDamage` Damage))

(event `self.CharacterDied`
  ;[0 0.5356 1] Example deathhandler
  (`KismetSystemLibrary.PrintString` "Enemy died!")
  (`self.DoDeath`))

(event `self.CharacterTookDamage`
  (bind _returnvalue (`GameplayStatics.SpawnEmitterAtLocation` "/Game/VFX/Particles/Particle_Hit.Particle_Hit" (+ (`SceneComponent.K2_GetComponentLocation` (`self.Mesh`)) (0.0 0.0 55.0))))
  (`SceneComponent.SetWorldScale3D` _returnvalue (1.3 1.3 1.3)))

(fn `UserConstructionScript`)