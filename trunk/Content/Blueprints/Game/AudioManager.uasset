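; Audio manager Blueprint that plays combat and pickup sounds and relays battle music fade requests.
; Gameplay events attach sounds to the involved actor's root, randomly choosing between two variants for deaths and attacks, with shouts layered on special attacks.
; BeginPlay binds menu, chat and escape UI events, but all UI handlers only print debug text.
; Potion, power-up and gold-drop sounds sit under a Deprecated label.
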(event `self.ReceiveBeginPlay`
  ;[0 0.333 1] BEGIN PLAY
  ;[1 1 1] MainMenu
  (add `self.UIMenuForward` (delegate `UIMenuForward_Event`))
  (add `self.UIMenuBackward` (delegate `UIMenuBackward_Event`))
  (add `self.UIChatMessage` (delegate `UIChatMessage_Event`))
  (add `self.UIEscapeMenu` (delegate `UIEscapeMenu_Event`)))

(event `self.UI_AreaClicked`
  (params (area :type "Actor Object Reference"))
  ;[1 1 1] MainMenu
  (bind _asga_ui_area (cast `GA_UI_Area` area))
  (`KismetSystemLibrary.PrintString` (`KismetStringLibrary.Concat_StrStr` "Click on: " (`KismetSystemLibrary.GetDisplayName` _asga_ui_area))))

(event `self.EnemyDied`
  (params (Enemy :type "GAEnemy Object Reference"))
  (bind _returnvalue (`self.K2_GetActorLocation` Enemy))
  (bind _returnvalue_2 (`self.K2_GetRootComponent` Enemy))
  ;[1 1 1] Combat
  (if (`KismetMathLibrary.RandomBool`)
    (`GameplayStatics.PlaySoundAttached` "/Game/Audio/SFX/orc_death_00.orc_death_00" _returnvalue_2 "None" _returnvalue "KeepWorldPosition")
    (else
      (`GameplayStatics.PlaySoundAttached` "/Game/Audio/SFX/orc_death_01.orc_death_01" _returnvalue_2 "None" _returnvalue))))

(event `self.CharacterDied`
  (params (Character :type "GACharacter Object Reference"))
  (bind _returnvalue (`self.K2_GetActorLocation` Character))
  (bind _returnvalue_2 (`self.K2_GetRootComponent` Character))
  ;[1 1 1] Combat
  (if (`KismetMathLibrary.RandomBool`)
    (`GameplayStatics.PlaySoundAttached` "/Game/Audio/SFX/player_death_00.player_death_00" _returnvalue_2 "None" _returnvalue)
    (else
      (`GameplayStatics.PlaySoundAttached` "/Game/Audio/SFX/player_death_01.player_death_01" _returnvalue_2 "None" _returnvalue))))

(event `self.UI_AreaHover`
  (params (area :type "Actor Object Reference"))
  ;[1 1 1] MainMenu
  (bind _asga_ui_area (cast `GA_UI_Area` area))
  (`KismetSystemLibrary.PrintString` (`KismetStringLibrary.Concat_StrStr` "Hover on: " (`KismetSystemLibrary.GetDisplayName` _asga_ui_area))))

(event `UIMenuForward_Event` :!signature `self.UIMenuForward`
  (params (area :type "Actor Object Reference"))
  ;[1 1 1] MainMenu
  (bind _asga_ui_area (cast `GA_UI_Area` area))
  (`KismetSystemLibrary.PrintString` (`KismetStringLibrary.Concat_StrStr` "Forward on: " (`KismetSystemLibrary.GetDisplayName` _asga_ui_area))))

(event `UIMenuBackward_Event` :!signature `self.UIMenuBackward`
  (params (area :type "Actor Object Reference"))
  ;[1 1 1] MainMenu
  (bind _asga_ui_area (cast `GA_UI_Area` area))
  (`KismetSystemLibrary.PrintString` (`KismetStringLibrary.Concat_StrStr` "Backward on: " (`KismetSystemLibrary.GetDisplayName` _asga_ui_area))))

(event `self.CharacterAttackedSimple`
  (params (Character :type "GACharacter Object Reference"))
  (bind _returnvalue (`self.K2_GetActorLocation` Character))
  (bind _returnvalue_2 (`self.K2_GetRootComponent` Character))
  ;[1 1 1] Combat
  (if (`KismetMathLibrary.RandomBool`)
    (`GameplayStatics.PlaySoundAttached` "/Game/Audio/SFX/player_simple_attack_00.player_simple_attack_00" _returnvalue_2 "None" _returnvalue)
    (else
      (`GameplayStatics.PlaySoundAttached` "/Game/Audio/SFX/player_attack_simple_01.player_attack_simple_01" _returnvalue_2 "None" _returnvalue))))

(event `self.CharacterStartedShardChanneling`
  (params (Character :type "GACharacter Object Reference"))
  ;[1 1 1] Combat
  (`GameplayStatics.PlaySoundAttached` "/Game/Audio/SFX/Shard_Channel_Weapon.Shard_Channel_Weapon" (`self.K2_GetRootComponent` Character) "None" (`self.K2_GetActorLocation` Character) "KeepWorldPosition" false 1.0))

(event `UIChatMessage_Event` :!signature `self.UIChatMessage`
  (params (area :type "Actor Object Reference"))
  ;[1 1 1] MainMenu
  (bind _asga_ui_area (cast `GA_UI_Area` area))
  (`KismetSystemLibrary.PrintString` (`KismetStringLibrary.Concat_StrStr` "Chat on: " (`KismetSystemLibrary.GetDisplayName` _asga_ui_area))))

(event `UIEscapeMenu_Event` :!signature `self.UIEscapeMenu`
  (params (area :type "Actor Object Reference"))
  ;[1 1 1] MainMenu
  (bind _asga_ui_area (cast `GA_UI_Area` area))
  (`KismetSystemLibrary.PrintString` (`KismetStringLibrary.Concat_StrStr` "Escape on: " (`KismetSystemLibrary.GetDisplayName` _asga_ui_area))))

(event `self.EnemyTookDamage`
  (params (Enemy :type "GAEnemy Object Reference"))
  ;[1 1 1] Combat
  (`GameplayStatics.PlaySoundAttached` "/Game/Audio/SFX/attack_hit.attack_hit" (`self.K2_GetRootComponent` Enemy) "None" (0.0 0.0 0.0) "EAttachLocation::KeepRelativeOffset" false 0.5))

(event `self.CharacterAttackedSpecial`
  (params (Character :type "GACharacter Object Reference"))
  (bind _returnvalue (`self.K2_GetActorLocation` Character))
  (bind _returnvalue_2 (`self.K2_GetRootComponent` Character))
  ;[1 1 1] Combat
  (if (`KismetMathLibrary.RandomBool`)
    (`GameplayStatics.PlaySoundAttached` "/Game/Audio/SFX/player_simple_attack_00.player_simple_attack_00" _returnvalue_2 "None" _returnvalue)
    (else
      (`GameplayStatics.PlaySoundAttached` "/Game/Audio/SFX/player_attack_simple_01.player_attack_simple_01" _returnvalue_2 "None" _returnvalue)))
  (if (`KismetMathLibrary.RandomBool`)
    (`GameplayStatics.PlaySoundAttached` "/Game/Audio/SFX/character_attack_shout_00.character_attack_shout_00" _returnvalue_2 "None" _returnvalue)
    (else
      (`GameplayStatics.PlaySoundAttached` "/Game/Audio/SFX/character_attack_shout_01.character_attack_shout_01" _returnvalue_2 "None" _returnvalue))))

(event `self.FadeInBattle`
  ;[1 1 1] Combat
  ;;[1 1 1] BGM
  (`self.FadeBattleIn`))

(event `self.FadeOutBattle`
  ;[1 1 1] Combat
  ;;[1 1 1] BGM
  (`self.FadeBattleOut`))

(event `self.CharacterUsedPotion`
  (params (Character :type "GACharacter Object Reference"))
  ;[1 1 1] Deprecated
  (`GameplayStatics.PlaySoundAttached` "/Game/Audio/SFX/potion_use.potion_use" (`self.K2_GetRootComponent` Character) "None" (0.0 0.0 0.0) "EAttachLocation::KeepRelativeOffset" false 1.0))

(event `self.PowerUpTaken`
  (params (PowerUp :type "GAPowerUp Object Reference"))
  ;[1 1 1] Combat
  (`GameplayStatics.PlaySoundAttached` "/Game/Audio/SFX/Powerup.PowerUp" (`self.K2_GetRootComponent` PowerUp) "None" (`self.K2_GetActorLocation` PowerUp) "KeepWorldPosition" false 1.0))

(event `self.EnemyDropedGold`
  (params (Enemy :type "GAEnemy Object Reference"))
  ;[1 1 1] Deprecated
  (`GameplayStatics.PlaySoundAttached` "/Game/Audio/SFX/drop_gold.drop_gold" (`self.K2_GetRootComponent` Enemy) "None" (0.0 0.0 0.0) "EAttachLocation::KeepRelativeOffset" false 1.0))

(fn `UserConstructionScript`)