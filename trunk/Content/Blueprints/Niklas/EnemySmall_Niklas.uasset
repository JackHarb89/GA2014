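; Small enemy character Blueprint that handles hit feedback and death cleanup.
; Taking damage spawns a scaled-up hit splatter particle at a fixed height above the mesh.
; Death, labeled as ragdoll, sets the dead flag and destroys the capsule.
; After a decay delay, the mesh switches to query-only collision, then the actor is destroyed shortly afterward.
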(event `self.CharacterDied`
  ;[1 1 1] Ragdoll
  (`KismetSystemLibrary.Delay` 0.0)
  (set `self.IsDead` true)
  (`ActorComponent.K2_DestroyComponent` (`self.CapsuleComponent`))
  (`KismetSystemLibrary.Delay` (`self.DecayDelay`))
  (`PrimitiveComponent.SetCollisionEnabled` (`self.Mesh`) "QueryOnly")
  (`KismetSystemLibrary.Delay` 2.0)
  (`self.K2_DestroyActor`))

(event `self.CharacterTookDamage`
  ;[1 1 1] Splatter Particle Effect
  (bind _returnvalue (`GameplayStatics.SpawnEmitterAtLocation` "/Game/VFX/Particles/Particle_Hit.Particle_Hit" (+ (`SceneComponent.K2_GetComponentLocation` (`self.Mesh`)) (0.0 0.0 55.0))))
  (`SceneComponent.SetWorldScale3D` _returnvalue (1.3 1.3 1.3)))

(fn `UserConstructionScript`)