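; Power-up pickup actor with a spinning mesh and three types: heal, invulnerability and one-hit.
; Construction script colors the light by type and snaps the pod to the surface below via a line trace.
; PowerUpTaken handles only cooldown, swapping in a type-specific dynamic material and switching off the light.
; A timeline feeds cooldown time to the heal material; after the delay, light restoration runs only for the heal type.
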(event `self.ReceiveBeginPlay`
  (bind (_direction _degrees) (`Timeline|rotate`)
    (:`Update`
      (`SceneComponent.SetRelativeRotation` (`self.PowerUp_Mesh`) (`KismetMathLibrary.MakeRot` 0.0 (* _degrees 25.0)) false))))

(event `self.PowerUpTaken`
  (bind _cooldown (`self.CoolDown`))
  (bind _poweruptype (`self.PowerUpType`))
  (if (not (`self.IsOnCooldown`))
    (if (== _poweruptype 0)
      (bind _returnvalue (`KismetMaterialLibrary.CreateDynamicMaterialInstance` "/Game/VFX/_VFX_Shader/mat_powerup_heal.mat_powerup_heal"))
      (`MaterialInstanceDynamic.SetScalarParameterValue` _returnvalue "ToggleFullGlow" 0.0)
      (set `self.IsOnCooldown` true)
      (`PrimitiveComponent.SetMaterial` (`self.PowerUp_Mesh`) 0 _returnvalue)
      (elif (== _poweruptype 1)
        (bind _returnvalue_2 (`KismetMaterialLibrary.CreateDynamicMaterialInstance` "/Game/VFX/_VFX_Shader/_VFX_Instances/invul.invul"))
        (`MaterialInstanceDynamic.SetScalarParameterValue` _returnvalue_2 "Opacity" 0.0)
        (set `self.IsOnCooldown` true)
        (`PrimitiveComponent.SetMaterial` (`self.PowerUp_Mesh`) 0 _returnvalue_2)
        (else
          (bind _returnvalue_3 (`KismetMaterialLibrary.CreateDynamicMaterialInstance` "/Game/VFX/_VFX_Shader/_VFX_Instances/onehit.onehit"))
          (`MaterialInstanceDynamic.SetScalarParameterValue` _returnvalue_3 "Opacity" 0.0)
          (set `self.IsOnCooldown` true)
          (`PrimitiveComponent.SetMaterial` (`self.PowerUp_Mesh`) 0 _returnvalue_3))))
    (`|ExecutionSequence`
      (:`then_0`
        (bind (_direction _time) (`Timeline|Timeline_0` :!via `PlayFromStart` :!label _label)
          (:`Update`
            (`MaterialInstanceDynamic.SetScalarParameterValue` _returnvalue "CustomTime" _time))))
      (:`then_1`
        (`MaterialInstanceDynamic.SetScalarParameterValue` _returnvalue "Cooldown Duration" _cooldown)
        (`KismetSystemLibrary.Delay` _cooldown)
        (`|ExecutionSequence`
          (:`then_0`
            (goto _label :!via `Stop`))
          (:`then_1`
            (goto _label :!via `SetNewTime`))
          (:`then_2`
            (set `self.IsOnCooldown` false)
            (`MaterialInstanceDynamic.SetScalarParameterValue` _returnvalue "ToggleFullGlow" 1.0)
            (if (not (!= _poweruptype 0))
              (`MaterialInstanceDynamic.SetScalarParameterValue` _returnvalue "Opacity" 1.0)
              (`MaterialInstanceDynamic.SetScalarParameterValue` _returnvalue_2 "Opacity" 1.0)
              (`LightComponent.SetBrightness` (`self.Light`) 10000.0)))))
      (:`then_2`
        (`LightComponent.SetBrightness` (`self.Light`) 0.0)))))

(fn `UserConstructionScript`
  (bind _poweruptype (`self.PowerUpType`))
  (bind _light (`self.Light`))
  (bind _pod (`self.Pod`))
  (bind _returnvalue (`SceneComponent.K2_GetComponentLocation` _pod))
  (if (== _poweruptype 1)
    (`LightComponent.SetLightColor` _light (struct :`R` 0.995 :`G` 0.814951 :`B` 0.213925 :`A` 1.0))
    (`PrimitiveComponent.SetMaterial` _pod 0 "/Game/VFX/_VFX_Shader/Heart_Inst.Heart_Inst" :!label _label)
    (bind _outhit (`KismetSystemLibrary.LineTraceSingle` _returnvalue (- _returnvalue (0.0 0.0 250.0)) "TraceTypeQuery1"))
    (`SceneComponent.SetWorldLocation` _pod (- (`GameplayStatics.BreakHitResult` _outhit) (0.0 0.0 5.0)) false)
    (elif (== _poweruptype 2)
      (`LightComponent.SetLightColor` _light (struct :`R` 0.192991 :`G` 0.292421 :`B` 0.995 :`A` 1.0))
      (goto _label)
      (elif (== _poweruptype 0)
        (`LightComponent.SetLightColor` _light (struct :`R` 0.245999 :`G` 1.0 :`B` 0.13 :`A` 1.0))
        (goto _label)))))