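; Player character Blueprint that handles combat visuals, an overhead name and health bar, and player hotkeys.
; Character events spawn attack, hit and regeneration particles, mostly oriented or offset by mesh yaw, plus a strength aura actor.
; Tick refreshes the name, scales the lifebar sprite from player 0's health ratio, and moves regen and aura effects with the character.
; Keys adjust walk speed, gamma and resolution, toggle HUD sections, and destroy shard hearts.
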(event `Key|MouseScrollDown`
  (bind _charactermovement (`self.CharacterMovement`))
  (:`Pressed`
    (set `CharacterMovementComponent.MaxWalkSpeed` (`KismetMathLibrary.FClamp` (+ (`CharacterMovementComponent.MaxWalkSpeed` _charactermovement) -500.0) 100.0 5000.0) _charactermovement)))

(event `Key|MouseScrollUp`
  (bind _charactermovement (`self.CharacterMovement`))
  (:`Pressed`
    (set `CharacterMovementComponent.MaxWalkSpeed` (`KismetMathLibrary.FClamp` (+ (`CharacterMovementComponent.MaxWalkSpeed` _charactermovement) 500.0) 100.0 5100.0) _charactermovement)))

(event `Key|MiddleMouseButton`
  (:`Pressed`
    (set `CharacterMovementComponent.MaxWalkSpeed` 600.0 (`self.CharacterMovement`))))

(event `self.CharacterAttackedSimple`
  ;[1 0 0] EVENTS
  ;;[1 1 1] Attack_Standard
  (`/Engine/EditorBlueprintResources/StandardMacros.IsValid` "PlayerCharacter_vincent"
    (:`Is Valid`
      (bind _returnvalue (`GameplayStatics.SpawnEmitterAtLocation` "/Game/VFX/Particles/Particle_Attack_Basic.Particle_Attack_Basic" (+ (* (`KismetMathLibrary.GetForwardVector` (`KismetMathLibrary.MakeRot` 0.0 (- (.yaw (`SceneComponent.K2_GetComponentRotation` (`self.Mesh`))) -90.0) (- (.roll (`SceneComponent.K2_GetComponentRotation` (`self.Mesh`))) -90.0))) 30.0) (+ (`self.K2_GetActorLocation`) (0.0 0.0 20.0))) (`KismetMathLibrary.MakeRot` 0.0 (- (.yaw (`SceneComponent.K2_GetComponentRotation` (`self.Mesh`))) -90.0) (- (.roll (`SceneComponent.K2_GetComponentRotation` (`self.Mesh`))) -90.0))))
      (set `self.Spawnedparticle` _returnvalue)
      (`AddComponent|RadialForceComponent_0` :`bManualAttachment` true :`RelativeTransform` (`KismetMathLibrary.MakeTransform` (`self.K2_GetActorLocation`))))))

(event `self.CharacterAttackedSpecial`
  ;[1 0 0] EVENTS
  ;;[1 1 1] Attack_Charged
  (`/Engine/EditorBlueprintResources/StandardMacros.IsValid` "PlayerCharacter_vincent"
    (:`Is Valid`
      (bind _returnvalue (`GameplayStatics.SpawnEmitterAtLocation` "/Game/VFX/Particles/Particle_Attack_Charged.Particle_Attack_Charged" (+ (`self.K2_GetActorLocation`) (0.0 0.0 20.0)) (`KismetMathLibrary.MakeRot` 0.0 (- (.yaw (`SceneComponent.K2_GetComponentRotation` (`self.Mesh`))) -90.0) (- (.roll (`SceneComponent.K2_GetComponentRotation` (`self.Mesh`))) -90.0))))
      (set `self.Spawnedparticle` _returnvalue))))

(event `self.CharacterFinishedRegeneration`
  (`ActorComponent.K2_DestroyComponent` (`self.SpawnedRegen`)))

(event `self.CharacterStartedRegeneration`
  ;[1 0 0] EVENTS
  ;;[1 1 1] Regen
  (`/Engine/EditorBlueprintResources/StandardMacros.IsValid` "/Game/VFX/Particles/P_Regen.P_Regen"
    (:`Is Valid`
      (bind _returnvalue (`GameplayStatics.SpawnEmitterAtLocation` "/Game/VFX/Particles/P_Regen.P_Regen" (+ (`self.K2_GetActorLocation`) (0.0 0.0 30.0))))
      (set `self.SpawnedRegen` _returnvalue))))

(event `self.CharacterTookDamage`
  ;[1 0 0] EVENTS
  ;;[1 1 1] Take_Damage
  (`/Engine/EditorBlueprintResources/StandardMacros.IsValid` "/Game/VFX/Particles/P_Regen.P_Regen"
    (:`Is Valid`
      (`GameplayStatics.SpawnEmitterAtLocation` "/Game/VFX/Particles/Particle_Hit.Particle_Hit" (+ (+ (+ (`self.K2_GetActorLocation`) (0.0 0.0 20.0)) (* (`KismetMathLibrary.GetForwardVector` (`KismetMathLibrary.MakeRot` 0.0 (- (.yaw (`SceneComponent.K2_GetComponentRotation` (`self.Mesh`))) -90.0) (- (.roll (`SceneComponent.K2_GetComponentRotation` (`self.Mesh`))) -90.0))) -5.0)) (0.0 0.0 10.0))))))

(event `Key|Z`
  ;[1 0 0] EVENTS
  ;;[1 1 1] Destroy_Heart
  (:`Pressed`
    (`/Engine/EditorBlueprintResources/StandardMacros.IsValid` "/Game/VFX/BP_Mockup_Shard_DM.BP_Mockup_Shard_DM"
      (:`Is Valid`
        (bind _outactors (`GameplayStatics.GetAllActorsOfClass` "/Game/VFX/BP_Mockup_Shard_DM.BP_Mockup_Shard_DM_C"))
        (for _array_element _outactors
          (bind _asbp_mockup_shard_dm_c (cast `/Game/VFX/BP_Mockup_Shard_DM` _array_element))
          (`/Game/VFX/BP_Mockup_Shard_DM.Destroy_Heart` _asbp_mockup_shard_dm_c))))))

(event `self.ReceiveTick`
  (params (DeltaSeconds :type "Float (single-precision)"))
  (bind _lifebar (`self.Lifebar`))
  ;[1 1 1] TICK
  ;[1 1 1] Update textrenderer above player mesh
  (`TextRenderComponent.SetText` (`self.UsernameRenderer`) (`self.UserName`))
  ;[1 1 1] Set current lifebar size
  (bind _asgacharacter (cast `GACharacter` (`GameplayStatics.GetPlayerCharacter` 0)))
  (`KismetArrayLibrary.Array_Set` (`MaterialBillboardComponent.Elements` (`self.Lifebar`)) 0 (make `MaterialBillboardComponent.MaterialSpriteElement` "/Game/VFX/Mat/Coin.Coin" null false 8.0 (* (/ (`GACharacter.HealthPoints` _asgacharacter) (`GACharacter.MaxHealth` _asgacharacter)) 32.0)) true)
  (`SceneComponent.ToggleVisibility` _lifebar true)
  (`SceneComponent.ToggleVisibility` _lifebar false)
  (`|ExecutionSequence`
    (:`then_0`
      (`/Engine/EditorBlueprintResources/StandardMacros.IsValid` "/Game/VFX/Particles/P_Regen.P_Regen"
        (:`Is Valid`
          (`SceneComponent.SetWorldLocation` (`self.SpawnedRegen`) (+ (+ (+ (`self.K2_GetActorLocation`) (0.0 0.0 20.0)) (* (`KismetMathLibrary.GetForwardVector` (`KismetMathLibrary.MakeRot` 0.0 (- (.yaw (`SceneComponent.K2_GetComponentRotation` (`self.Mesh`))) -90.0) (- (.roll (`SceneComponent.K2_GetComponentRotation` (`self.Mesh`))) -90.0))) -5.0)) (0.0 0.0 10.0)) false))))
    (:`then_1`
      (`/Engine/EditorBlueprintResources/StandardMacros.IsValid` (stale `self.CharacterActivatedAura` _returnvalue)
        (:`Is Valid`
          (`self.K2_SetActorLocation` (stale `self.CharacterActivatedAura` _returnvalue) (- (`self.K2_GetActorLocation`) (0.0 0.0 50.0)) false))))))

(event `self.CharacterActivatedAura`
  ;[1 1 1] TICK
  (bind _returnvalue (`|SpawnActorFromClass` "/Game/Blueprints/Peddy/BP_Aura_Strength.BP_Aura_Strength_C" (`KismetMathLibrary.MakeTransform` (- (`self.K2_GetActorLocation`) (0.0 0.0 50.0))) true)))

(event `self.CharacterDeactivatedAura`
  ;[1 1 1] TICK
  (`/Engine/EditorBlueprintResources/StandardMacros.IsValid` (stale `self.CharacterActivatedAura` _returnvalue)
    (:`Is Valid`
      (`self.K2_DestroyActor` (stale `self.CharacterActivatedAura` _returnvalue)))))

(event `Key|PageUp`
  (:`Pressed`
    (set `self.Increase?` true)
    (`self.Setresxy` (`self.Increase?`))))

(event `Key|I`
  ;[1 1 1] Toggle inventory
  (:`Pressed`
    (bind _asga_hud_bp_c (cast `/Game/UI/Classes/GA_HUD_BP` (`PlayerController.GetHUD` (`GameplayStatics.GetPlayerController` 0))))
    (bind _returnvalue (`GA_HUD.getSection` _asga_hud_bp_c "inventory"))
    (switch `int` _returnvalue
      (:`0`
        (set `self.showInventory` true))
      (:`1`
        (set `self.showInventory` false)))
    (`GA_HUD.toggleSection` _asga_hud_bp_c "inventory" (`self.showInventory`))))

(event `Key|PageDown`
  (:`Pressed`
    (set `self.Increase?` false)))

(event `Key|Add`
  (:`Pressed`
    (`self.Gamma+` (`self.Increment`))))

(event `Key|Subtract`
  (:`Pressed`
    (`self.Gamma-` (`self.Increment`))))

(event `Key|Z`
  ;[1 1 1] Toggle escapemenu
  (:`Pressed`
    (bind _asga_hud_bp_c (cast `/Game/UI/Classes/GA_HUD_BP` (`PlayerController.GetHUD` (`GameplayStatics.GetPlayerController` 0))))
    (bind _returnvalue (`GA_HUD.getSection` _asga_hud_bp_c "escapemenu"))
    (switch `int` _returnvalue
      (:`0`
        (set `self.showEscapemenu` true))
      (:`1`
        (set `self.showEscapemenu` false)))
    (`GA_HUD.toggleSection` _asga_hud_bp_c "escapemenu" (`self.showEscapemenu`))))

(event `Key|P`
  ;[1 1 1] Toggle stats
  (:`Pressed`
    (set `self.showStats` true)
    (bind _asga_hud_bp_c (cast `/Game/UI/Classes/GA_HUD_BP` (`PlayerController.GetHUD` (`GameplayStatics.GetPlayerController` 0)) :!label _label))
    (`GA_HUD.toggleSection` _asga_hud_bp_c "sessioninfo" (`self.showStats`)))
  (:`Released`
    (set `self.showStats` false)
    (goto _label)))

(fn `Gamma+`
  (params (Increment :type "Float (double-precision)"))
  (set `self.Gamma` (`KismetMathLibrary.FClamp` (+ (`self.Gamma`) (`self.Increment`)) 0.2 4.2))
  (`KismetSystemLibrary.ExecuteConsoleCommand` (`KismetStringLibrary.Concat_StrStr` "gamma " (`KismetStringLibrary.Conv_DoubleToString` (`self.Gamma`)))))

(fn `Gamma-`
  (params (Increment :type "Float (double-precision)"))
  (set `self.Gamma` (`KismetMathLibrary.FClamp` (- (`self.Gamma`) (`self.Increment`)) 0.2 4.2))
  (`KismetSystemLibrary.ExecuteConsoleCommand` (`KismetStringLibrary.Concat_StrStr` "gamma " (`KismetStringLibrary.Conv_DoubleToString` (`self.Gamma`)))))

(fn `Setresxy`
  (params (`Increase/Decrease` :type Boolean))
  (bind _returnvalue (`KismetStringLibrary.Concat_StrStr` "setres " (`self.1920x1200`)))
  (bind _returnvalue_2 (`KismetStringLibrary.Concat_StrStr` "setres " (`self.1920x1080`)))
  (if true
    (`KismetSystemLibrary.ExecuteConsoleCommand` _returnvalue (`GameplayStatics.GetPlayerController` 0))
    (set `self.Resolution` _returnvalue)
    (else
      (`KismetSystemLibrary.ExecuteConsoleCommand` _returnvalue_2 (`GameplayStatics.GetPlayerController` 0))
      (set `self.Resolution` _returnvalue_2))))

(fn `UserConstructionScript`)