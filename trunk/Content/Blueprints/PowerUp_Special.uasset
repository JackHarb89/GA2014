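; PowerUp_Special is a child power-up Blueprint whose appearance follows PowerUpType: an armor helmet with the Invul material or a one-hit mesh.
; The construction script calls its parent, then sets the mesh, also applying material and doubled scale for the helmet only.
; The PowerUpFinishedCoolDown event reapplies mesh and material for either type when cooldown ends.
; Pickup and effect logic are absent from these graphs.
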(event `self.PowerUpFinishedCoolDown`
  (bind _poweruptype (`self.PowerUpType`))
  (bind _powerup_mesh (`self.PowerUp_Mesh`))
  (if (== _poweruptype 1)
    (`StaticMeshComponent.SetStaticMesh` _powerup_mesh "/Game/Meshes/Items/item_armor_helmet.item_armor_helmet")
    (`PrimitiveComponent.SetMaterial` _powerup_mesh 0 "/Game/VFX/_VFX_Shader/_VFX_Instances/invul.invul")
    (elif (== _poweruptype 2)
      (`StaticMeshComponent.SetStaticMesh` _powerup_mesh "/Game/Meshes/SG_powerup_onehit.SG_powerup_onehit")
      (`PrimitiveComponent.SetMaterial` _powerup_mesh 0 "/Game/VFX/_VFX_Shader/_VFX_Instances/onehit.onehit"))))

(fn `UserConstructionScript`
  (bind _poweruptype (`self.PowerUpType`))
  (bind _powerup_mesh (`self.PowerUp_Mesh`))
  (`parent.UserConstructionScript`)
  (if (== _poweruptype 1)
    (`StaticMeshComponent.SetStaticMesh` _powerup_mesh "/Game/Meshes/Items/item_armor_helmet.item_armor_helmet")
    (`PrimitiveComponent.SetMaterial` _powerup_mesh 0 "/Game/VFX/_VFX_Shader/_VFX_Instances/invul.invul")
    (`SceneComponent.SetWorldScale3D` _powerup_mesh (2.0 2.0 2.0))
    (elif (== _poweruptype 2)
      (`StaticMeshComponent.SetStaticMesh` _powerup_mesh "/Game/Meshes/SG_powerup_onehit.SG_powerup_onehit"))))