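; bp_Cube is a cube that displays the player's simple-attack cooldown through its material.
; Its startcooldown event ignores calls during a cooldown, then creates a dynamic instance of the attack spell material and sets duration and on-cooldown parameters from GACharacter's SimpleAttackCoolDown.
; A timeline feeds a CustomTime parameter to the material until a delay of that length stops it and clears the cooldown state.
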(event `startcooldown`
  (if (not (`self.IsOnCooldown_AttackSimple`))
    (set `self.IsOnCooldown_AttackSimple` true)
    (bind _returnvalue (`PrimitiveComponent.CreateDynamicMaterialInstance` (`self.Cube`) 0 "/Game/Material/Instances/mat_spell_attacksimple.mat_spell_attacksimple"))
    (`|ExecutionSequence`
      (:`then_0`
        (bind (_direction _time) (`Timeline|TL_CustomTime` :!via `PlayFromStart` :!label _label)
          (:`Update`
            (`MaterialInstanceDynamic.SetScalarParameterValue` _returnvalue "CustomTime" _time))))
      (:`then_1`
        (bind _asgacharacter (cast `GACharacter` (`GameplayStatics.GetPlayerCharacter` 0)))
        (bind _simpleattackcooldown (`GACharacter.SimpleAttackCoolDown` _asgacharacter))
        (`MaterialInstanceDynamic.SetScalarParameterValue` _returnvalue "Cooldown Duration" _simpleattackcooldown)
        (`MaterialInstanceDynamic.SetScalarParameterValue` _returnvalue "IsOnCooldown" 1.0)
        (`KismetSystemLibrary.Delay` _simpleattackcooldown)
        (`|ExecutionSequence`
          (:`then_0`
            (goto _label :!via `Stop`))
          (:`then_1`
            (`MaterialInstanceDynamic.SetScalarParameterValue` _returnvalue "IsOnCooldown" 0.0)
            (set `self.IsOnCooldown_AttackSimple` false)))))))

(fn `UserConstructionScript`)