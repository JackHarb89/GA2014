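; Sword item actor, built around a Chest component, that settles onto the ground and can be turned in small yaw steps.
; On authority, the construction script traces down from Chest's relative location, used as a world position, moves Chest to the impact point and calls SetDropAnimationFinished.
; Event AA sets the actor rotation to Chest's world rotation with a slight yaw offset, so repeated calls spin it.
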(event `AA`
  (`self.SetActorRotation` (`KismetMathLibrary.MakeRot` (.pitch (`SceneComponent.K2_GetComponentRotation` (`self.Chest`))) (+ (.yaw (`SceneComponent.K2_GetComponentRotation` (`self.Chest`))) 1.2) (.roll (`SceneComponent.K2_GetComponentRotation` (`self.Chest`))))))

(fn `UserConstructionScript`
  (bind _chest (`self.Chest`))
  (bind _relativelocation (`SceneComponent.RelativeLocation` _chest))
  (`/Engine/EditorBlueprintResources/ActorMacros.Switch Has Authority`
    (:`Authority`
      (bind _outhit (`KismetSystemLibrary.LineTraceSingle` _relativelocation (- _relativelocation (0.0 0.0 3000.0)) "TraceTypeQuery1" true))
      (`SceneComponent.SetWorldLocation` _chest (`.ImpactPoint` (`GameplayStatics.BreakHitResult` _outhit)) false)
      (`self.SetDropAnimationFinished`))))